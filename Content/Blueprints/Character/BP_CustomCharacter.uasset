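; Player character Blueprint that registers drone movement and world interaction input mapping bundles with MyPlayerController on BeginPlay.
; Tick prints debug state from the current movement and lock-on components, and the move input events only print their direction.
; GetVectorsForMovement returns camera-based forward, right and up vectors, using a quaternion to align them to gravity when grounded.
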(event OnComponentHit(Box)
  (params (HitComponent :type Primitive%20Component%20Object%20Reference) (OtherActor :type Actor%20Object%20Reference) (OtherComp :type Primitive%20Component%20Object%20Reference) (NormalImpulse :type Vector :default "0, 0, 0") (Hit :type Hit%20Result%20Structure%20%28by%20ref%29)))

(event Input|EnhancedActionEvents|EnhancedInputActionIA_PC_MoveRight
  (params (ActionValue :type Float%20%28double-precision%29) (ElapsedSeconds :type Float%20%28double-precision%29) (TriggeredSeconds :type Float%20%28double-precision%29) (InputAction :type Input%20Action%20Object%20Reference :default "/Game/Input/Movement/Drone_Movement/IA_PC_MoveRight.IA_PC_MoveRight"))
  (Development|PrintString (Utilities|String|ToString(Text) (Utilities|Text|FormatText "is adding {text}" (Utilities|Text|ToText(String) (select (< ActionValue 0.0) "left" "right")))) true false "(R=0.000000,G=0.660000,B=1.000000,A=1.000000)" 0.0))

(event Input|EnhancedActionEvents|EnhancedInputActionIA_PC_MoveUp
  (params (ActionValue :type Float%20%28double-precision%29) (ElapsedSeconds :type Float%20%28double-precision%29) (TriggeredSeconds :type Float%20%28double-precision%29) (InputAction :type Input%20Action%20Object%20Reference :default "/Game/Input/Movement/Drone_Movement/IA_PC_MoveUp.IA_PC_MoveUp"))
  (Development|PrintString (Utilities|String|ToString(Text) (Utilities|Text|FormatText "is adding {text}" (Utilities|Text|ToText(String) (select (< ActionValue 0.0) "down" "up")))) true false "(R=0.000000,G=0.660000,B=1.000000,A=1.000000)" 0.0))

(event Input|EnhancedActionEvents|EnhancedInputActionIA_PC_MoveForward
  (params (ActionValue :type Float%20%28double-precision%29) (ElapsedSeconds :type Float%20%28double-precision%29) (TriggeredSeconds :type Float%20%28double-precision%29) (InputAction :type Input%20Action%20Object%20Reference :default "/Game/Input/Movement/Drone_Movement/IA_PC_MoveForward.IA_PC_MoveForward"))
  (Development|PrintString (Utilities|String|ToString(Text) (Utilities|Text|FormatText "is adding {text}" (Utilities|Text|ToText(String) (select (< ActionValue 0.0) "backward" "forward")))) true false "(R=0.000000,G=0.660000,B=1.000000,A=1.000000)" 0.0))

(event EventTick
  (params (DeltaSeconds :type Float%20%28single-precision%29))
  (bind _current_movement_comp (Variables|Default|GetCurrent_Movement_Comp))
  (bind _current_movement_comp_2 (Variables|Default|GetCurrent_Movement_Comp))
  (Development|PrintString (Utilities|String|ToString(Vector) (Variables|/Script/Custom_Movement.DroneMovementComponent|GetMovementInput _current_movement_comp_2)) true false "(R=1.000000,G=0.685655,B=0.000000,A=1.000000)" 0.0)
  (Development|PrintString (Utilities|String|SelectString "is boosting" "stoped boosting" (Class|DroneMovementComponent|IsBoosting _current_movement_comp_2)) true false "(R=0.000000,G=0.367140,B=1.000000,A=1.000000)" 0.0)
  (Development|PrintString (Utilities|String|SelectString "is moving" "is not moving" (Class|DroneMovementComponent|IsMoving _current_movement_comp)) true false "(R=1.000000,G=0.529962,B=0.440013,A=1.000000)" 0.0)
  (Development|PrintString (Utilities|String|ToString(Vector) (Class|DroneMovementComponent|GetVelocity _current_movement_comp)) true false "(R=0.055236,G=0.461238,B=1.000000,A=1.000000)" 0.0)
  (Development|PrintString (Utilities|String|ToString(Vector) (Class|DroneMovementComponent|GetDecelVelocity _current_movement_comp)) true false "(R=1.000000,G=0.067083,B=0.166763,A=1.000000)" 0.0)
  (Development|PrintString (Utilities|String|SelectString "is Locked on" "is not Locked on" (Class|DroneMovementComponent|IsLockedon _current_movement_comp)) true false "(R=1.000000,G=0.067083,B=0.166763,A=1.000000)" 0.0)
  (Development|PrintString (Utilities|GetDisplayName (Class|TargetLockonComponent|GetLockedTarget (Variables|Default|GetLockOn_Comp))) true false "(R=0.000000,G=0.796248,B=1.000000,A=1.000000)" 0.0))

(event EventBeginPlay
  (bind _asmy_player_controller (Utilities|Casting|CastToMyPlayerController (Pawn|GetController))
    (:then
      (Variables|Default|SetAs%20My%20Player%20Controller _asmy_player_controller)
      (Utilities|FlowControl|Sequence
        (:then_0
          ;[0.15 0.15 0.15 0.5] Movement IMC_B
          (bind _output_get (Variables|Default|SetMovement%20IMC_B (Utilities|Struct|MakeIMC_Bundle "Drone Movement IMC_B" self "Movement_IMC" (Variables|Default|GetMovement%20IMC%20B%20GP%20IMC) (Variables|Default|GetMovement%20IMC%20B%20PC%20IMC) 0)))
          (Class|MyPlayerController|SetMovementIMCBundles (Variables|Default|GetAs%20My%20Player%20Controller) _output_get)
          (Class|MyPlayerController|AddMappingandBindActions (Variables|Default|GetAs%20My%20Player%20Controller) _output_get))
        (:then_1
          ;[0.15 0.15 0.15 0.5] World Interaction IMC_B
          (bind _output_get_2 (Variables|Default|SetWorld%20Interaction%20IMC_B (Utilities|Struct|MakeIMC_Bundle "World_Interaction_IMC_B" self "World_Interaction_IMC" (Variables|Default|GetWorld%20Interaction%20IMC%20B%20GP%20IMC) (Variables|Default|GetWorld%20Interaction%20IMC%20B%20PC%20IMC) 0)))
          (Class|MyPlayerController|SetWorldInteractionIMCBundles (Variables|Default|GetAs%20My%20Player%20Controller) _output_get_2)
          (Class|MyPlayerController|AddMappingandBindActions (Variables|Default|GetAs%20My%20Player%20Controller) _output_get_2))))
    (:CastFailed
      (Development|PrintString "Error, Controller casting Failed" true false "(R=1.000000,G=0.000000,B=0.048242,A=1.000000)" 1e+01))))

(fn ConstructionScript)

(fn GetVectorsforMovement
  (bind _returnvalue (Game|GetPlayerCameraManager 0))
  (bind _gravity_direction (Variables|Default|Getgravity%20direction))
  (bind _is_on_ground (Variables|Default|Getis%20on%20ground))
  (bind _returnvalue_2 (Camera|GetCameraRotation _returnvalue))
  (bind _returnvalue_3 (Math|Vector|Normalize _gravity_direction))
  (bind _returnvalue_4 (Math|Conversions|ToQuaternion(Rotator) _returnvalue_2))
  (bind _returnvalue_5 (Math|Vector|GetUpVector _returnvalue_2))
  (bind _returnvalue_6 (* _returnvalue_5 -1))
  (bind _returnvalue_7 (Class|KismetMathLibrary|QuatFindBetweenNormals _returnvalue_6 _returnvalue_3))
  (bind _returnvalue_8 (* _returnvalue_4 _returnvalue_7))
  (bind _returnvalue_9 (Class|KismetMathLibrary|QuatRotator _returnvalue_8))
  (bind _returnvalue_10 (select _is_on_ground _returnvalue_9 _returnvalue_2))
  (return (Math|Vector|GetForwardVector _returnvalue_10) (Math|Vector|GetRightVector _returnvalue_10) (Math|Vector|GetUpVector _returnvalue_10)))
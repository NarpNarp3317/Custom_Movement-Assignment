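; Player controller Blueprint that sets up Enhanced Input mapping contexts for UI interaction and menu controls.
; On BeginPlay it builds one bundle for each, combining a name, itself, the context, its GP and PC variants and a priority.
; Each bundle is stored in a variable and passed to AddMappingAndBindActions to register the mappings and bind actions.
; Tick and the construction script are empty.
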(event EventBeginPlay
  (Utilities|FlowControl|Sequence
    (:then_0
      ;[0.15 0.15 0.15 0.5] UI_Interaction IMC
      (bind _output_get (Variables|Default|SetUI_Interaction_IMC_B (Utilities|Struct|MakeIMC_Bundle "UI_Interaction" self "UI_Interaction_IMC" (Variables|Default|GetUI_Interaction_IMC_GP) (Variables|Default|GetUI_Interaction_IMC_PC) 0)))
      (Class|MyPlayerController|SetUIInteractionIMCBundles _output_get)
      (Class|MyPlayerController|AddMappingandBindActions _output_get))
    (:then_1
      ;[0.15 0.15 0.15 0.5] Menu IMC
      (bind _output_get_2 (Variables|Default|SetMenu_IMC_B (Utilities|Struct|MakeIMC_Bundle "Menu Interaction" self "Menu_IMC" (Variables|Default|GetMenu_IMC_GP) (Variables|Default|GetMenu_IMC_PC) 0)))
      (Class|MyPlayerController|SetMenuIMCBundles _output_get_2)
      (Class|MyPlayerController|AddMappingandBindActions _output_get_2))))

(event EventTick
  (params (DeltaSeconds :type Float%20%28single-precision%29)))

(fn ConstructionScript)